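; First-person weapon actor that fires projectiles for its owning BP_FirstPerson character.
; BeginPlay caches the owner cast to BP_FirstPerson.
; Fire plays the rifle montage on the owner's arms, a sound, and a muzzle flash attached to the Arrow component.
; It then spawns the projectile at the Arrow's location using the first-person camera's rotation, so shots follow the view rather than the muzzle's orientation.
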(event `self.ReceiveBeginPlay`
  (bind _asbp_first_person (cast `/Game/FirstPerson/Blueprints/BP_FirstPerson` (`self.GetOwner`)))
  (set `self.As BP FPSSimple` _asbp_first_person))

(event `Fire`
  (bind _arrow (`self.Arrow`))
  (bind _as_bp_fpssimple (`self.As BP FPSSimple`))
  (bind (_returnvalue_location _returnvalue_rotation) (`KismetMathLibrary.BreakTransform` (`SceneComponent.GetRelativeTransform` _arrow)))
  (`AnimInstance.Montage_Play` (`SkeletalMeshComponent.GetAnimInstance` (`/Game/FirstPerson/Blueprints/BP_FirstPerson.Arms` _as_bp_fpssimple)) "/Game/FirstPerson/Arms/NewAnimations/FP_Rifle_Shoot_Montage.FP_Rifle_Shoot_Montage" 1.0 "MontageLength" 0.0 true)
  (`GameplayStatics.PlaySoundAtLocation` (`self.Sound`) (`self.K2_GetActorLocation`) (struct) 1.0 1.0 0.05 null null null null) ; Play firing sound
  (`NiagaraFunctionLibrary.SpawnSystemAttached` "/Game/Effects/P_MuzzleFlash.P_MuzzleFlash" _arrow "None" _returnvalue_location _returnvalue_rotation "KeepRelativeOffset" true)
  (`|SpawnActorFromClass` (`self.ProjectileClass`) (`KismetMathLibrary.MakeTransform` (`SceneComponent.K2_GetComponentLocation` (`self.Arrow`)) (`SceneComponent.K2_GetComponentRotation` (`/Game/FirstPerson/Blueprints/BP_FirstPerson.FirstPersonCamera` _as_bp_fpssimple))) "AdjustIfPossibleButDontSpawnIfColliding" "OverrideRootScale" null null) ; Spawn projectile
)

(fn `UserConstructionScript`)
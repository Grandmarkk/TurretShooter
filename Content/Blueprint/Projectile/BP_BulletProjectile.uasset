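; BP_BulletProjectile is a bullet projectile that damages what it hits and triggers a physics field at the impact.
; On Hit it spawns spark particles and an FS_MasterField actor aligned to the surface normal, then fires that field's CETrigger.
; It applies fixed damage through the other actor's HealthComponent, if one exists, then destroys itself.
; A DamagedAmount function returns zero and is not used in the hit logic.
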(event `self.ReceiveHit`
  (params (MyComp :type "PrimitiveComponent Object Reference") (Other :type "Actor Object Reference") (OtherComp :type "PrimitiveComponent Object Reference") (bSelfMoved :type Boolean) (HitLocation :type "Vector Structure") (HitNormal :type "Vector Structure") (NormalImpulse :type "Vector Structure") (Hit :type "HitResult Structure (by ref)"))
  (bind (_bblockinghit _binitialoverlap _time _distance _location _impactpoint _normal _impactnormal) (`GameplayStatics.BreakHitResult` Hit))
  (bind _returnvalue (`self.GetComponentByClass` Other "/Script/TurretShooter.HealthComponent"))
  (`NiagaraFunctionLibrary.SpawnSystemAtLocation` "/Game/Effects/P_ProjectileSparks.P_ProjectileSparks" HitLocation (`KismetMathLibrary.Conv_VectorToRotator` HitNormal))
  (bind _returnvalue_2 (`|SpawnActorFromClass` "/Engine/EditorResources/FieldNodes/FS_MasterField.FS_MasterField_C" (`KismetMathLibrary.MakeTransform` _impactpoint (`KismetMathLibrary.Conv_VectorToRotator` _impactnormal)) "Undefined" "MultiplyWithRoot" null null))
  (`/Engine/EditorResources/FieldNodes/FS_MasterField.CE_Trigger` _returnvalue_2)
  (`/Engine/EditorBlueprintResources/StandardMacros.IsValid` _returnvalue
    (:`Is Valid`
      (`HealthComponent.ApplyDamage` :`self` _returnvalue :`DamageAmount` 5.0))
    (:`Is Not Valid`
      _))
  (`self.K2_DestroyActor`))

(fn `DamagedAmount`
  (returns (DamageAmount :type Integer))
  (return 0))

(fn `UserConstructionScript`)
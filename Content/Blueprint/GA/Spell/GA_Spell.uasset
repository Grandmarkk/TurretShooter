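; GA_Spell is a Gameplay Ability that casts a projectile spell from the avatar's hand in the camera's facing direction.
; On activation it spawns the Projectile class just ahead of the static mesh's right-hand socket, oriented along the camera forward vector, and plays Sound there.
; It then force-commits only the cooldown, without a cost commit, and ends immediately.
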(event `self.K2_ActivateAbility`
  (bind _returnvalue (`self.GetAvatarActorFromActorInfo`))
  (bind _returnvalue_2 (`SceneComponent.GetForwardVector` (`Actor.GetComponentByClass` _returnvalue "/Script/Engine.CameraComponent")))
  (bind _returnvalue_3 (+ (`SceneComponent.GetSocketLocation` (`Actor.GetComponentByClass` _returnvalue "/Script/Engine.StaticMeshComponent") "hand_r") (* _returnvalue_2 (100.0 100.0 100.0))))
  (`|SpawnActorFromClass` (`self.Projectile`) (`KismetMathLibrary.MakeTransform` _returnvalue_3 (`KismetMathLibrary.Conv_VectorToRotator` _returnvalue_2)) "Undefined" "MultiplyWithRoot" null null)
  (`GameplayStatics.PlaySoundAtLocation` (`self.Sound`) _returnvalue_3 (struct) 1.0 1.0 0.0 null null null null)
  (`self.K2_CommitAbilityCooldown` false true)
  (`self.K2_EndAbility`))